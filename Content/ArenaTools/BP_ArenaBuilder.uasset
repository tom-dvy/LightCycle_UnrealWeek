(fn `Build`
  (bind _returnvalue (`self.GetTransform`))
  (bind _floor (`self.Floor`))
  (bind _grid (`self.Grid`))
  (bind _grid_2 (`self.Grid`))
  (bind _grid_3 (`self.Grid`))
  (bind _grid_4 (`self.Grid`))
  (bind _cellsize (`/Game/ArenaTools/PDA_ArenaGrid.CellSize` _grid_4))
  (bind _cellsize_2 (`/Game/ArenaTools/PDA_ArenaGrid.CellSize` _grid_3))
  (bind _returnvalue_2 (* (`/Game/ArenaTools/PDA_ArenaGrid.Width` _grid_4) _cellsize))
  (bind _returnvalue_3 (* (`/Game/ArenaTools/PDA_ArenaGrid.Height` _grid_4) _cellsize))
  (bind _returnvalue_4 (/ (`/Game/ArenaTools/PDA_ArenaGrid.CellSize` _grid_2) 100.0))
  (`|ExecutionSequence`
    (:`then_0`
      ; Nettoyage
      (`/Engine/EditorBlueprintResources/StandardMacros.IsValid` (`self.Grid`)
        (:`Is Valid`
          (`InstancedStaticMeshComponent.ClearInstances` (`self.ISM_Walls`))
          (`InstancedStaticMeshComponent.ClearInstances` (`self.ISM_PowerUpMarkers`))
          (`InstancedStaticMeshComponent.ClearInstances` (`self.ISM_SpawnMarkers`))
          (`KismetArrayLibrary.Array_Clear` (`self.SpawnTransforms`))
          (`KismetArrayLibrary.Array_Clear` (`self.PowerUpTransforms`)))
        (:`Is Not Valid`
          (`KismetSystemLibrary.PrintString` "Grid invalide, STOP"))))
    (:`then_1`
      ; Config du sol
      (`SceneComponent.SetRelativeScale3D` _floor (`KismetMathLibrary.MakeVector` (/ _returnvalue_2 100.0) (/ _returnvalue_3 100.0) 1.0))
      (`SceneComponent.K2_SetRelativeLocation` _floor (`KismetMathLibrary.MakeVector` (/ _returnvalue_2 2.0) (/ _returnvalue_3 2.0)) false false)
      ; Boucle Y
      (for _index (range (`/Game/ArenaTools/PDA_ArenaGrid.Height` _grid))
        ; Boucle X
        (for _index_2 (range (`/Game/ArenaTools/PDA_ArenaGrid.Width` _grid))
          (bind _cell (`/Game/ArenaTools/PDA_ArenaGrid.GetCell` _grid _index_2 _index))
          (switch `/Game/ArenaTools/E_ArenaCell` _cell
            (:`NewEnumerator1`
              ; Wall
              (`InstancedStaticMeshComponent.AddInstance` (`self.ISM_Walls`) (`KismetMathLibrary.MakeTransform` (+ (`KismetMathLibrary.MakeVector` 0.0 0.0 (/ (`self.WallHeight`) 2.0)) (`/Game/ArenaTools/PDA_ArenaGrid.CellToLocal` _grid_2 _index_2 _index)) (struct) (`KismetMathLibrary.MakeVector` _returnvalue_4 _returnvalue_4 (/ (`self.WallHeight`) 100.0))) false))
            (:`NewEnumerator2`
              (bind _returnvalue_5 (`KismetMathLibrary.MakeTransform` (`/Game/ArenaTools/PDA_ArenaGrid.CellToLocal` (`self.Grid`) _index_2 _index) (`KismetMathLibrary.MakeRotator` (.roll (`KismetMathLibrary.FindLookAtRotation` (`KismetMathLibrary.TransformLocation` _returnvalue (`/Game/ArenaTools/PDA_ArenaGrid.CellToLocal` _grid_3 _index_2 _index)) (`KismetMathLibrary.TransformLocation` _returnvalue (`KismetMathLibrary.MakeVector` (/ (* (`/Game/ArenaTools/PDA_ArenaGrid.Width` _grid_3) _cellsize_2) 2.0) (/ (* (`/Game/ArenaTools/PDA_ArenaGrid.Height` _grid_3) _cellsize_2) 2.0))))) (- (.pitch (`KismetMathLibrary.FindLookAtRotation` (`KismetMathLibrary.TransformLocation` _returnvalue (`/Game/ArenaTools/PDA_ArenaGrid.CellToLocal` _grid_3 _index_2 _index)) (`KismetMathLibrary.TransformLocation` _returnvalue (`KismetMathLibrary.MakeVector` (/ (* (`/Game/ArenaTools/PDA_ArenaGrid.Width` _grid_3) _cellsize_2) 2.0) (/ (* (`/Game/ArenaTools/PDA_ArenaGrid.Height` _grid_3) _cellsize_2) 2.0))))) 90.0) (* (`KismetMathLibrary.Round` (/ (.yaw (`KismetMathLibrary.FindLookAtRotation` (`KismetMathLibrary.TransformLocation` _returnvalue (`/Game/ArenaTools/PDA_ArenaGrid.CellToLocal` _grid_3 _index_2 _index)) (`KismetMathLibrary.TransformLocation` _returnvalue (`KismetMathLibrary.MakeVector` (/ (* (`/Game/ArenaTools/PDA_ArenaGrid.Width` _grid_3) _cellsize_2) 2.0) (/ (* (`/Game/ArenaTools/PDA_ArenaGrid.Height` _grid_3) _cellsize_2) 2.0))))) 90.0)) 90))))
              ; Spawn
              (`KismetArrayLibrary.Array_Add` (`self.SpawnTransforms`) _returnvalue_5)
              (`InstancedStaticMeshComponent.AddInstance` (`self.ISM_SpawnMarkers`) _returnvalue_5 false))
            (:`NewEnumerator3`
              (bind _returnvalue_6 (`KismetMathLibrary.MakeTransform` (`/Game/ArenaTools/PDA_ArenaGrid.CellToLocal` (`self.Grid`) _index_2 _index) (`KismetMathLibrary.MakeRotator` 0.0 -90.0)))
              ; PowerUp
              (`KismetArrayLibrary.Array_Add` (`self.PowerUpTransforms`) _returnvalue_6)
              (`InstancedStaticMeshComponent.AddInstance` (`self.ISM_PowerUpMarkers`) _returnvalue_6 false))))))))

(fn `Rebuild`
  (`self.Build`))

(fn `UserConstructionScript`
  (`self.Build`))