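; Player controller for a two-player light cycle arena, routing shared-keyboard steering to each player's BP_LightCycle pawn.
; Only the controller at index 0 adds the IMC_Default Enhanced Input mapping context on BeginPlay.
; Separate move actions for each player write TargetTurnInput on player pawn 0 or 1 while triggered and reset it to zero on completion.
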(event `self.ReceiveBeginPlay`
  (if (== self (`GameplayStatics.GetPlayerController` 0))
    (`EnhancedInputSubsystemInterface.AddMappingContext` (subsystem `EnhancedInputLocalPlayerSubsystem`) "/Game/Input/IMC_Default.IMC_Default" 0 (struct))))

(event `EnhancedInput|/Game/Input/Actions/IA_Move_P1`
  (params (ActionValue :type "Float (double-precision)") (ElapsedSeconds :type "Float (double-precision)") (TriggeredSeconds :type "Float (double-precision)") (InputAction :type "InputAction Object Reference" :default "/Game/Input/Actions/IA_Move_P1.IA_Move_P1"))
  (bind _returnvalue (`GameplayStatics.GetPlayerPawn` 0))
  ; Input Joueur 1 (Q & D)
  (:`Triggered`
    (bind _asbp_light_cycle (cast `/Game/LightCycle/Blueprint/BP_LightCycle` _returnvalue))
    (set `/Game/LightCycle/Blueprint/BP_LightCycle.TargetTurnInput` ActionValue _asbp_light_cycle))
  (:`Completed`
    (bind _asbp_light_cycle_2 (cast `/Game/LightCycle/Blueprint/BP_LightCycle` _returnvalue))
    (set `/Game/LightCycle/Blueprint/BP_LightCycle.TargetTurnInput` 0.0 _asbp_light_cycle_2)))

(event `EnhancedInput|/Game/Input/Actions/IA_Move_P2`
  (params (ActionValue :type "Float (double-precision)") (ElapsedSeconds :type "Float (double-precision)") (TriggeredSeconds :type "Float (double-precision)") (InputAction :type "InputAction Object Reference" :default "/Game/Input/Actions/IA_Move_P2.IA_Move_P2"))
  (bind _returnvalue (`GameplayStatics.GetPlayerPawn` 1))
  ; Input Joueur 2 (Flèche droite & Gauche)
  (:`Triggered`
    (bind _asbp_light_cycle (cast `/Game/LightCycle/Blueprint/BP_LightCycle` _returnvalue))
    (set `/Game/LightCycle/Blueprint/BP_LightCycle.TargetTurnInput` ActionValue _asbp_light_cycle))
  (:`Completed`
    (bind _asbp_light_cycle_2 (cast `/Game/LightCycle/Blueprint/BP_LightCycle` _returnvalue))
    (set `/Game/LightCycle/Blueprint/BP_LightCycle.TargetTurnInput` 0.0 _asbp_light_cycle_2)))

(fn `UserConstructionScript`)