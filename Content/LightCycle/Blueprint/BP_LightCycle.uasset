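; Player light cycle in a Tron-style game that drives forward constantly, steers with smoothed turn input and kills cycles crossing its trail.
; Tick records distance-spaced path points; a looping timer line-traces between them to detect victims.
; Trail or environment hits call DeathManager and report scores to BP_MyGameMode.
; DeathManager plays slow-motion death effects, requests respawn and resets every cycle's path and Niagara trail.
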(event `self.ReceiveBeginPlay`
  (`GameplayStatics.PlaySound2D` "/Game/LightCycle/Song/S_spawn.S_spawn" 1.0 1.0 0.0 null null)
  (set `self.MyNiagaraRef` (`self.Niagara`))
  (set `self.SpawnTransform` (`self.GetTransform`))
  (set `self.IsAlive` true)
  (`KismetSystemLibrary.K2_SetTimerDelegate` (delegate `TriggerCollisionCheck`) 0.05 true))

(event `TriggerCollisionCheck`
  (`self.CheckCollision`))

(event `self.ReceiveTick`
  (params (DeltaSeconds :type "Float (single-precision)"))
  (bind _returnvalue (`self.K2_GetActorLocation`))
  (bind _pathpoint (`self.PathPoint`))
  (bind _pathpoint_2 (`self.PathPoint`))
  (bind _isalive (`self.IsAlive`))
  (if _isalive
    (`|ExecutionSequence`
      (:`then_0`
        ; Move automatically forward
        (`self.K2_AddActorWorldOffset` (* (`self.GetActorForwardVector`) (* (`self.Speed`) DeltaSeconds)) true))
      (:`then_1`
        ; Rotate
        (set `self.CurrentTurnInput` (`KismetMathLibrary.FInterpTo` (`self.CurrentTurnInput`) (`self.TargetTurnInput`) (`GameplayStatics.GetWorldDeltaSeconds`) 10.0))
        (`self.K2_AddActorWorldRotation` (`KismetMathLibrary.MakeRotator` 0.0 0.0 (* (* (`self.CurrentTurnInput`) (`self.RotationSpeed`)) DeltaSeconds))))
      (:`then_2`
        (if _isalive
          ; Point Gestion
          (if (== (`KismetArrayLibrary.Array_Length` _pathpoint_2) 0)
            (`KismetArrayLibrary.Array_Add` _pathpoint_2 _returnvalue)
            (if (>= (`KismetArrayLibrary.Array_Length` _pathpoint) 500)
              (`KismetArrayLibrary.Array_Remove` _pathpoint))
            (elif (> (`KismetMathLibrary.Vector_Distance` _returnvalue (`|GetArrayItem` _pathpoint_2 (`KismetArrayLibrary.Array_LastIndex` _pathpoint_2))) (`self.MinDistance`))
              (`KismetArrayLibrary.Array_Add` (`self.PathPoint`) (`self.K2_GetActorLocation`)))))))))

(event `self.Collider.OnComponentHit`
  (params (HitComponent :type "PrimitiveComponent Object Reference") (OtherActor :type "Actor Object Reference") (OtherComp :type "PrimitiveComponent Object Reference") (NormalImpulse :type "Vector Structure") (Hit :type "HitResult Structure (by ref)"))
  ; Collisions avec environnement
  (`self.DeathManager` false)
  (bind _asbp_my_game_mode (cast `/Game/LightCycle/Blueprint/BP_MyGameMode` (`GameplayStatics.GetGameMode`)))
  (`/Game/LightCycle/Blueprint/BP_MyGameMode.ManageScore` _asbp_my_game_mode self null))

(fn `CheckCollision`
  (returns (OutHit :type "HitResult Structure") (IsCollide :type Boolean))
  (for (_array_element _array_index) (`self.PathPoint`)
    (if (< _array_index (- (`KismetArrayLibrary.Array_Length` (`self.PathPoint`)) 1))
      (bind (_outhit _returnvalue) (`KismetSystemLibrary.LineTraceSingle` _array_element (`|GetArrayItem` (`self.PathPoint`) (+ _array_index 1)) "TraceTypeQuery1" true (`|MakeArray` self :!type "Actor Object Reference") "None" false))
      (if _returnvalue
        (bind _asbp_light_cycle (cast `/Game/LightCycle/Blueprint/BP_LightCycle` (`.HitActor` (`GameplayStatics.BreakHitResult` _outhit))))
        ; Mort
        (bind _output_get (set `/Game/LightCycle/Blueprint/BP_LightCycle.IsAlive` false _asbp_light_cycle))
        (`self.DeathManager` _asbp_light_cycle _output_get)
        ; Gestion Score
        (bind _asbp_my_game_mode (cast `/Game/LightCycle/Blueprint/BP_MyGameMode` (`GameplayStatics.GetGameMode`)))
        (`/Game/LightCycle/Blueprint/BP_MyGameMode.ManageScore` _asbp_my_game_mode _asbp_light_cycle self)
        (return _outhit true))
      (else
        (break))))
  (return (struct) false))

(fn `DeathManager`
  (params (IsAlive :type Boolean :default true))
  (bind _myniagararef (`self.MyNiagaraRef`))
  (bind _spawnedtrailsegments (`self.SpawnedTrailSegments`))
  (if (not IsAlive)
    (`|ExecutionSequence`
      (:`then_0`
        (set `self.Speed` 0.0)
        ; Player Dead
        (`self.SetActorEnableCollision` false)
        (`self.SetActorHiddenInGame` true)
        (for _array_element _
          (`self.DisableInput` (`GameplayStatics.GetPlayerController` _array_element)))
        (`GameplayStatics.PlaySound2D` "/Game/LightCycle/Song/S_death.S_death" 1.0 1.0 0.0 null null)
        (`GameplayStatics.SetGlobalTimeDilation` 0.05)
        (`NiagaraFunctionLibrary.SpawnSystemAtLocation` (`self.System Template`) (`self.K2_GetActorLocation`))
        (`KismetSystemLibrary.K2_SetTimer` null "StartExplosion" 0.06)
        (`SkeletalMeshComponent.Stop` (`self.Beat_anim4`))
        (`NiagaraComponent.ReinitializeSystem` _myniagararef)
        (`ActorComponent.Deactivate` _myniagararef)
        (for _array_element_2 _spawnedtrailsegments
          (`self.K2_DestroyActor` _array_element_2))
        (`KismetArrayLibrary.Array_Clear` _spawnedtrailsegments))
      (:`then_1`
        ; Respawn
        (bind _asbp_my_game_mode (cast `/Game/LightCycle/Blueprint/BP_MyGameMode` (`GameplayStatics.GetGameMode`)))
        (`/Game/LightCycle/Blueprint/BP_MyGameMode.RespawnTimer` _asbp_my_game_mode)
        (set `self.IsAlive` true)
        (bind _outactors (`GameplayStatics.GetAllActorsOfClass` "BP_LightCycle_C"))
        (for _array_element_3 _outactors
          (`KismetArrayLibrary.Array_Clear` (`/Game/LightCycle/Blueprint/BP_LightCycle.PathPoint` _array_element_3))
          (bind _niagara (`/Game/LightCycle/Blueprint/BP_LightCycle.Niagara` _array_element_3))
          (`NiagaraComponent.ReinitializeSystem` _niagara)
          (`ActorComponent.Activate` _niagara false))
        (`SkeletalMeshComponent.Play` (`self.Beat_anim4`) true)))))

(fn `StartExplosion`
  (`GameplayStatics.SetGlobalTimeDilation` 1.0))

(fn `UserConstructionScript`)