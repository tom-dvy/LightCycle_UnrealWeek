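; Game mode for the LightCycle game that handles the score HUD, kill scoring and cycle respawns.
; BeginPlay creates the score display widget, and ManageScore takes a point from suicides or gives one to the killer, stored in each PlayerState, then refreshes it.
; RespawnTimer waits briefly, then RespawnManager resets every light cycle at once: spawn transform, visibility, collision, speed, and input by player controller index.
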(event `RespawnTimer`
  (`KismetSystemLibrary.K2_SetTimerDelegate` (delegate `Respawn`) 0.5))

(event `Respawn`
  (`self.RespawnManager`))

(event `self.ReceiveBeginPlay`
  (bind _returnvalue (`|CreateWidget` "/Game/LightCycle/Blueprint/WBP_ScoreDisplay.WBP_ScoreDisplay_C"))
  (set `self.ScoreHUD_Ref` _returnvalue)
  (`UserWidget.AddToViewport` _returnvalue 0))

(fn `ManageScore`
  (params (Victim :type "/Game/LightCycle/Blueprint/BP_LightCycle Object Reference") (Killer :type "/Game/LightCycle/Blueprint/BP_LightCycle Object Reference"))
  (if (== Victim Killer)
    ; Suicide
    (bind _asbp_my_player_state (cast `/Game/LightCycle/Blueprint/BP_MyPlayerState` (`Controller.PlayerState` (`Pawn.GetController` Victim))))
    (set `/Game/LightCycle/Blueprint/BP_MyPlayerState.CurrentScore` (- (`/Game/LightCycle/Blueprint/BP_MyPlayerState.CurrentScore` _asbp_my_player_state) 1) _asbp_my_player_state)
    (`/Game/LightCycle/Blueprint/WBP_ScoreDisplay.UpdateScores` (`self.ScoreHUD_Ref`))
    (else
      ; Mort par un autre joueur
      (bind _asbp_my_player_state_2 (cast `/Game/LightCycle/Blueprint/BP_MyPlayerState` (`Controller.PlayerState` (`Pawn.GetController` Killer))))
      (set `/Game/LightCycle/Blueprint/BP_MyPlayerState.CurrentScore` (+ (`/Game/LightCycle/Blueprint/BP_MyPlayerState.CurrentScore` _asbp_my_player_state_2) 1) _asbp_my_player_state_2)
      (`/Game/LightCycle/Blueprint/WBP_ScoreDisplay.UpdateScores` (`self.ScoreHUD_Ref`)))))

(fn `RespawnManager`
  (bind _outactors (`GameplayStatics.GetAllActorsOfClass` "/Game/LightCycle/Blueprint/BP_LightCycle.BP_LightCycle_C"))
  (for (_array_element _array_index) _outactors
    (`self.K2_SetActorTransform` _array_element (`/Game/LightCycle/Blueprint/BP_LightCycle.SpawnTransform` _array_element) false true)
    (`self.SetActorHiddenInGame` _array_element false)
    (`self.SetActorEnableCollision` _array_element true)
    (`self.EnableInput` _array_element (`GameplayStatics.GetPlayerController` _array_index))
    (set `/Game/LightCycle/Blueprint/BP_LightCycle.Speed` 1200.0 _array_element)))

(fn `UserConstructionScript`)